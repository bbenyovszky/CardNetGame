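; Playing card actor for a multiplayer card game that shows its face, moves to given transforms and forwards clicks to GamePS.
; Dynamic materials take textures from the ZsuCardMap data table, keyed by suit and rank for the front.
; The RelevantTo rep-notify refreshes the front, which shows a back texture to players for whom the card is not relevant.
; MoveTo teleports with yaw-flip correction, as its timeline lerp is disconnected.
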(event Custom|SetFrontMaterial
  (bind _cardfrontmesh (Variables|Default|GetCardFrontMesh))
  ;[1 1 1] Setting the Front Material based on the Card's Deck, Color, and Rank
  (bind _returnvalue (Rendering|Material|CreateDynamicMaterialInstance _cardfrontmesh 0 (Rendering|Material|GetMaterial _cardfrontmesh 0) :!class /Script/Engine.PrimitiveComponent))
  (switch Utilities|FlowControl|Switch|SwitchonEDeck (Variables|Default|GetDeck)
    (:NewEnumerator0
      (bind _returnvalue_2 (Utilities|GetDataTableRow "/Game/Assets/Decks/ZsuCard/ZsuCardMap.ZsuCardMap" (select (CallFunction|IsRelevant) (Utilities|String|StringToName (Utilities|String|ToString(Text) (Utilities|Text|FormatText "{Color}_{Rank}" (Math|Byte|MakeLiteralByte (Variables|Default|GetSuit)) (Math|Byte|MakeLiteralByte (Variables|Default|GetRank))))) (Utilities|String|StringToName (Utilities|String|ToString(Text) (Utilities|Text|FormatText "B{Type}" (Class|KismetSystemLibrary|MakeLiteralInteger))))))
        (:then
          (Rendering|Material|SetTextureParameterValue _returnvalue "FrontTexture" (.texture _returnvalue_2)))))))

(event Custom|SetBackMaterial
  (bind _cardbackmesh (Variables|Default|GetCardBackMesh))
  ;[1 1 1] Setting the Back Material based on the Card's Deck
  (bind _returnvalue (Rendering|Material|CreateDynamicMaterialInstance _cardbackmesh 0 (Rendering|Material|GetMaterial _cardbackmesh 0) :!class /Script/Engine.PrimitiveComponent))
  (switch Utilities|FlowControl|Switch|SwitchonEDeck (Variables|Default|GetDeck)
    (:NewEnumerator0
      (bind _returnvalue_2 (Utilities|GetDataTableRow "/Game/Assets/Decks/ZsuCard/ZsuCardMap.ZsuCardMap" (Utilities|String|StringToName (Utilities|String|ToString(Text) (Utilities|Text|FormatText "B{Type}" (Class|KismetSystemLibrary|MakeLiteralInteger)))))
        (:then
          (Rendering|Material|SetTextureParameterValue _returnvalue "BackTexture" (.texture _returnvalue_2)))))))

(event Custom|RefreshMaterials
  (CallFunction|SetFrontMaterial)
  (CallFunction|SetBackMaterial))

(event Custom|MoveTo
  (params (To :type Transform))
  (bind (_location _rotation _scale) (Math|Transform|BreakTransform To))
  ;[1 1 1] Moves the card smoothly to its new position
  (bind _output_get (Variables|Default|SetLastPos (Transformation|GetRelativeTransform (Variables|Default|GetDefaultSceneRoot))))
  (Transformation|SetRelativeTransform (Variables|Default|GetDefaultSceneRoot) (select (< 9e+01 (Math|Float|%(Float) (Math|Float|Absolute(Float) (- (.yaw _rotation) (.yaw (.Rotation (Math|Transform|BreakTransform _output_get))))) 1.8e+02)) (Math|Transform|MakeTransform _location (Math|Rotator|MakeRotator (.roll _rotation) (- 0.0 (.pitch _rotation)) (+ (.yaw _rotation) 1.8e+02)) _scale) To) false true))

(event EventBeginPlay
  (CallFunction|RefreshMaterials))

(event MouseInput|EventActorOnClicked
  (params (ButtonPressed :type Key%20Structure :default "AnyKey"))
  ;[1 1 1] Registrates clicks and sends it to the PlayerState
  (Default|CardClicked (.AsGame%20PS (Utilities|Casting|CastToGamePS (Variables|/Script/Engine.Controller|GetPlayerState (Game|GetPlayerController 0)))) self (== ButtonPressed "LeftMouseButton")))

(fn ConstructionScript)

(fn OneRankAway
  (params (From :type Card%20BP%20Object%20Reference))
  (bind _rank (Variables|CardBP_C|GetRank From))
  (bind _rank_2 (Variables|Default|GetRank))
  (bind _returnvalue (- _rank 1))
  (return (or (== _returnvalue (Class|KismetMathLibrary|PercentByteByte (+ _rank_2 0) 13)) (== _returnvalue (Class|KismetMathLibrary|PercentByteByte (+ _rank_2 11) 13)))))

(fn OnRepRelevantto
  (CallFunction|SetFrontMaterial))

(fn GetSuit
  (return (Variables|Default|GetSuit)))

(fn GetRank
  (return (Variables|Default|GetRank)))

(fn IsRelevant
  (bind _relevantto (Variables|Default|GetRelevantTo))
  (if (== -1 _relevantto)
    _
    (elif (== _relevantto (Variables|/Game/Blueprints/AllLevels/GamePC.GamePC_C|GetMyNumber (.AsGame%20PC (Utilities|Casting|CastToGamePC (Game|GetPlayerController 0)))))
      _
      (else
        (return false))))
  (return true))