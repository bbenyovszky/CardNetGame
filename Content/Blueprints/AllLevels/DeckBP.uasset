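; DeckBP is a card pile actor that spawns standard, joker or German-suit decks of CardBP actors and handles shuffling, sorting, adding and drawing.
; An ordered Cards array drives the stack, with Rearrange moving attached cards to thickness-based height offsets.
; FaceUp sets card flip and which array end is the top.
; Draws detach cards, additions pass on RelevantTo, and Sort buckets by suit and rank, jokers last.
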(event Custom|Rearrange
  (bind _cards (Variables|Default|GetCards))
  (for (_array_element _array_index) _cards
    (Default|Moveto _array_element (Math|Transform|MakeTransform (* (Math|Vector|GetUpVector (Variables|Default|GetDefaultSceneRoot)) (* (Math|Integer|SelectInt _array_index (- (Utilities|Array|LastIndex _cards) _array_index) (Variables|Default|GetFaceUp?)) (Variables|Default|GetCardThickness))) (Variables|Default|GetDefRot)))))

(event Custom|Shuffle
  (Utilities|Array|Shuffle (Variables|Default|GetCards)))

(event Custom|Clear
  (bind _cards (Variables|Default|GetCards))
  (for _array_element _cards
    (Actor|DestroyActor _array_element))
  (Utilities|Array|Clear _cards))

(event Custom|RefreshCards
  (for _array_element (Variables|Default|GetCards)
    (Default|SetFrontMaterial _array_element)))

(event Custom|AddCards
  (params (Cards :type Array%20of%20Card%20BP%20Object%20References) (ToTop :type Boolean))
  (for _array_element Cards
    (Transformation|AttachComponentToComponent _array_element (Variables|Default|GetDefaultSceneRoot) "None" "KeepWorld" "KeepWorld" "KeepWorld" false)
    (Variables|/Game/Blueprints/AllLevels/CardBP.CardBP_C|SetRelevantTo _array_element (Variables|Default|GetRelevantTo))
    (if (Math|Boolean|Equal(Boolean) ToTop (Variables|Default|GetFaceUp?))
      (Utilities|Array|Add (Variables|Default|GetCards) _array_element)
      (else
        (Utilities|Array|Insert (Variables|Default|GetCards) _array_element))))
  (CallFunction|Rearrange))

(event Custom|StandardDeck
  (params (Deck :type Array%20of%20EDeck%20Enums) (w/Joker? :type Boolean) (Shuffle :type Boolean))
  (bind _array (Utilities|Array|MakeArray "NewEnumerator0" "NewEnumerator1" "NewEnumerator2" "NewEnumerator3"))
  (CallFunction|AddDeckOf Deck _array (Utilities|Array|MakeArray "NewEnumerator1" "NewEnumerator2" "NewEnumerator3" "NewEnumerator4" "NewEnumerator5" "NewEnumerator6" "NewEnumerator7" "NewEnumerator8" "NewEnumerator9" "NewEnumerator10" "NewEnumerator11" "NewEnumerator12" "NewEnumerator13") (and (not w/Joker?) Shuffle))
  (if w/Joker?
    (CallFunction|AddDeckOf Deck _array (Utilities|Array|MakeArray "NewEnumerator0") Shuffle)))

(event Custom|GermanSuit
  (params (Deck :type EDeck%20Enum) (Shuffle :type Boolean))
  (CallFunction|AddDeckOf (Utilities|Array|MakeArray Deck) (Utilities|Array|MakeArray "NewEnumerator0" "NewEnumerator1" "NewEnumerator2" "NewEnumerator3") (Utilities|Array|MakeArray "NewEnumerator7" "NewEnumerator8" "NewEnumerator9" "NewEnumerator10" "NewEnumerator11" "NewEnumerator12" "NewEnumerator13" "NewEnumerator1") Shuffle))

(event Custom|AddCard
  (params (Card :type Card%20BP%20Object%20Reference) (ToTop :type Boolean))
  (bind _cards (Variables|Default|GetCards))
  (Transformation|AttachComponentToComponent Card (Variables|Default|GetDefaultSceneRoot) "None" "KeepWorld" "KeepWorld" "SnapToTarget" false)
  (Variables|/Game/Blueprints/AllLevels/CardBP.CardBP_C|SetRelevantTo Card (Variables|Default|GetRelevantTo))
  (if (Math|Boolean|Equal(Boolean) ToTop (Variables|Default|GetFaceUp?))
    (Utilities|Array|Add _cards Card)
    (else
      (Utilities|Array|Insert _cards Card)))
  (if ToTop
    (Default|Moveto Card (Math|Transform|MakeTransform (* (Math|Vector|GetUpVector (Variables|Default|GetDefaultSceneRoot)) (* (Utilities|Array|LastIndex (Variables|Default|GetCards)) (Variables|Default|GetCardThickness))) (Variables|Default|GetDefRot)))
    (else
      (CallFunction|Rearrange))))

(event Custom|AddDeckOf
  (params (Deck :type Array%20of%20EDeck%20Enums) (Suit :type Array%20of%20ESuit%20Enums) (Rank :type Array%20of%20ERank%20Enums) (Shuffle :type Boolean))
  (for _array_element Deck
    (for _array_element_2 Suit
      (for _array_element_3 Rank
        (bind _returnvalue (Game|SpawnActorfromClass "/Game/Blueprints/AllLevels/CardBP.CardBP_C" (Transformation|GetWorldTransform (Variables|Default|GetDefaultSceneRoot)) "Undefined" 0 _array_element _array_element_2 _array_element_3))
        (Variables|/Game/Blueprints/AllLevels/CardBP.CardBP_C|SetRelevantTo _returnvalue (Variables|Default|GetRelevantTo))
        (Transformation|AttachComponentToComponent (Variables|/Game/Blueprints/AllLevels/CardBP.CardBP_C|GetDefaultSceneRoot _returnvalue) (Variables|Default|GetDefaultSceneRoot) "None" "SnapToTarget" "SnapToTarget" "SnapToTarget" false)
        (Utilities|Array|Add (Variables|Default|GetCards) _returnvalue)
        (if (not (Variables|Default|GetFaceUp?))
          (Transformation|AddRelativeRotation (Variables|/Game/Blueprints/AllLevels/CardBP.CardBP_C|GetDefaultSceneRoot _returnvalue) "180.000000, 0, 0" false false)))))
  (if Shuffle
    (CallFunction|Shuffle))
  (CallFunction|Rearrange))

(event EventBeginPlay
  (Components|Activation|Deactivate (Variables|Default|GetSpotLight)))

(fn ConstructionScript
  (Rendering|SetVisibility (Variables|Default|GetSpotLight) (Variables|Default|GetLightOn) false)
  (Rendering|Components|TextRender|SetText (Variables|Default|GetDeckInfo) (Variables|EngineInfo|GetDeckInfoText))
  (Variables|Default|SetDefRot (Math|Rotator|MakeRotator (.Roll (Math|Rotator|BreakRotator (Variables|Default|GetDefRot))) (+ (.Pitch (Math|Rotator|BreakRotator (Variables|Default|GetDefRot))) (Math|Float|SelectFloat 0.0 1.8e+02 (Variables|Default|GetFaceUp?))) (.Yaw (Math|Rotator|BreakRotator (Variables|Default|GetDefRot))))))

(fn GetCard
  (params (FromTop :type Boolean))
  (bind _cards (Variables|Default|GetCards))
  (bind _faceup_ (Variables|Default|GetFaceUp?))
  (bind _returnvalue (Utilities|Array|LastIndex _cards))
  (bind _returnvalue_2 (Class|KismetMathLibrary|XORBoolean FromTop _faceup_))
  (bind _returnvalue_3 (Math|Integer|SelectInt 0 _returnvalue _returnvalue_2))
  (bind _output_get (LocalVariables|SetChosenOne (Utilities|Array|Get(acopy) _cards _returnvalue_3)))
  (Transformation|DetachFromActor _output_get "KeepWorld" "KeepWorld" "KeepRelative")
  (Utilities|Array|RemoveIndex (Variables|Default|GetCards) _returnvalue_3)
  (if FromTop
    _
    (else
      (CallFunction|Rearrange)))
  (return _output_get))

(fn Empty
  (return (not (Math|Conversions|ToBoolean(Integer) (Utilities|Array|Length (Variables|Default|GetCards))))))

(fn CheckTopCard
  (bind _cards (Variables|Default|GetCards))
  (return (Utilities|Array|Get(acopy) _cards (Math|Integer|SelectInt (Utilities|Array|LastIndex _cards) 0 (Variables|Default|GetFaceUp?)))))

(fn Sort
  (for _array_element (Variables|Default|GetCards)
    (Utilities|Array|Add (select (Utilities|Enum|NotEqual(Enum) (Default|GetRank _array_element) "NewEnumerator0") (Utilities|Select :Index (Default|GetSuit _array_element) :NewEnumerator0 (LocalVariables|Get0) :NewEnumerator1 (LocalVariables|Get1) :NewEnumerator2 (LocalVariables|Get2) :NewEnumerator3 (LocalVariables|Get3)) (LocalVariables|GetJ)) _array_element))
  (Utilities|Array|Clear (Variables|Default|GetCards))
  (for _index (range 0 3)
    (bind _enumvalue (|ForEachERank)
      (:LoopBody
        (if (Utilities|Enum|NotEqual(Enum) _enumvalue "NewEnumerator0")
          (for _array_element_2 (Utilities|Select :Index _index :Option%200 (LocalVariables|Get0) :Option%201 (LocalVariables|Get1) :Option%202 (LocalVariables|Get2) :Option%203 (LocalVariables|Get3))
            (if (Utilities|Enum|Equal(Enum) (Default|GetRank _array_element_2) _enumvalue)
              (Utilities|Array|Add (Variables|Default|GetCards) _array_element_2)))))))
  (Utilities|Array|AppendArray (Variables|Default|GetCards) (LocalVariables|GetJ)))

(fn NumOfCards
  (return (Utilities|Array|Length (Variables|Default|GetCards))))

(fn GetCards
  (params (Amount :type Integer) (FromTop :type Boolean))
  (bind _cards (Variables|Default|GetCards))
  (bind _faceup_ (Variables|Default|GetFaceUp?))
  (bind _returnvalue (Utilities|Array|LastIndex _cards))
  (bind _returnvalue_2 (Class|KismetMathLibrary|XORBoolean FromTop _faceup_))
  (bind _returnvalue_3 (Math|Integer|SelectInt 0 _returnvalue _returnvalue_2))
  (bind _item (Utilities|Array|Get(acopy) _cards _returnvalue_3))
  (Utilities|FlowControl|ForLoopwithBreak 1 Amount :!label _label
    (:LoopBody
      (if (!= (Utilities|Array|Length _cards) 0)
        (Utilities|Array|Add (LocalVariables|GetChosenOnes) _item)
        (Transformation|DetachFromActor _item "KeepWorld" "KeepWorld" "KeepRelative")
        (Utilities|Array|RemoveIndex (Variables|Default|GetCards) _returnvalue_3)
        (else
          (goto _label Break))))
    (:Completed
      (if FromTop
        _
        (else
          (CallFunction|Rearrange)))
      (return (LocalVariables|GetChosenOnes)))))

(fn ContainsThis
  (params (This :type Card%20BP%20Object%20Reference))
  (return (Utilities|Array|FindItem (Variables|Default|GetCards) This)))

(fn OnRepCards)