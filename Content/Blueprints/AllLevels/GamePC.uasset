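; GamePC is a player controller that handles per-player setup, the escape menu and quitting the game.
; InitialSetup stores the player number in MyNumber, forwards it to the GamePS player state, then calls ClientSetup, which stores it again and enables Game and UI input.
; Escape or Q toggles a lazily created, cached EscapeMenuWB widget, and ExitGame quits.
; MyNumber has a RepNotify, but its handler is empty.
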(event Custom|ClientSetup
  (params (PlayerNumber :type Integer))
  (Variables|Default|SetMyNumber PlayerNumber)
  (Input|SetInputModeGameandUI self 0 "DoNotLock" false))

(event Custom|ExitGame
  (Game|QuitGame 0 "Quit"))

(event Custom|InitialSetup
  (params (PlayerNumber :type Integer))
  (bind _output_get (Variables|Default|SetMyNumber PlayerNumber))
  (Default|InitialSetup (.AsGame%20PS (Utilities|Casting|CastToGamePS (Variables|GetPlayerState))) PlayerNumber)
  (CallFunction|ClientSetup _output_get))

(event Input|KeyboardEvents|Escape
  (params (Key :type Key%20Structure :default "AnyKey"))
  (:Pressed
    (Utilities|IsValid (Variables|Default|GetEscapeMenu)
      (:Is%20Valid
        _)
      (:Is%20Not%20Valid
        (bind _returnvalue (UserInterface|CreateWidget "/Game/UI/Game/EscapeMenuWB.EscapeMenuWB_C" self))
        (bind _output_get (Variables|Default|SetEscapeMenu _returnvalue))))
    (if (UserInterface|Viewport|IsinViewport _output_get)
      (Widget|RemovefromParent _output_get)
      (else
        (UserInterface|Viewport|AddtoViewport _output_get 0)))))

(event Input|KeyboardEvents|Q
  (params (Key :type Key%20Structure :default "AnyKey"))
  (:Pressed
    (Utilities|IsValid (Variables|Default|GetEscapeMenu)
      (:Is%20Valid
        _)
      (:Is%20Not%20Valid
        (bind _returnvalue (UserInterface|CreateWidget "/Game/UI/Game/EscapeMenuWB.EscapeMenuWB_C" self))
        (bind _output_get (Variables|Default|SetEscapeMenu _returnvalue))))
    (if (UserInterface|Viewport|IsinViewport _output_get)
      (Widget|RemovefromParent _output_get)
      (else
        (UserInterface|Viewport|AddtoViewport _output_get 0)))))

(fn ConstructionScript)

(fn OnRepMyNumber)