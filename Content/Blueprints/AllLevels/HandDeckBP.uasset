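; HandDeckBP is a card hand that holds card actors and lays them out in a centered row.
; Added cards are attached to the root, given the deck's RelevantTo value, then sorted and rearranged.
; Rearrange moves each card to an evenly spaced local X offset, and OnRepCards repeats it when the replicated array updates.
; GetCardAt detaches and removes a card before closing the gap, while CheckCardAt only reads it.
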(event EventRearrange
  (bind _cards (Variables|Default|GetCards))
  (for (_array_element _array_index) _cards
    (Utilities|IsValid _array_element
      (:Is%20Valid
        (Default|Moveto _array_element (Math|Transform|MakeTransform (Math|Vector|MakeVector (* (Variables|Default|GetWidth) (+ (Math|Conversions|ToFloat(Integer) _array_index) (* (Utilities|Array|LastIndex _cards) -0.5))) 0.0 0.0) (Variables|Default|GetDefRot) "1,1,1.000000"))))))

(event EventAddCard
  (params (Card :type Card%20BP%20Object%20Reference) (ToTop :type Boolean))
  (Transformation|AttachComponentToComponent Card (Variables|Default|GetDefaultSceneRoot) "None" "KeepWorld" "KeepWorld" "SnapToTarget" false)
  (Variables|/Game/Blueprints/AllLevels/CardBP.CardBP_C|SetRelevantTo Card (Variables|Default|GetRelevantTo))
  (Utilities|Array|Add (Variables|Default|GetCards) Card)
  (CallFunction|Sort)
  (CallFunction|Rearrange))

(event EventAddCards
  (params (Cards :type Array%20of%20Card%20BP%20Object%20References) (ToTop :type Boolean))
  (for _array_element Cards
    (Transformation|AttachComponentToComponent _array_element (Variables|Default|GetDefaultSceneRoot) "None" "KeepWorld" "KeepWorld" "SnapToTarget" false)
    (Variables|/Game/Blueprints/AllLevels/CardBP.CardBP_C|SetRelevantTo _array_element (Variables|Default|GetRelevantTo))
    (Utilities|Array|Add (Variables|Default|GetCards) _array_element))
  (CallFunction|Sort)
  (CallFunction|Rearrange))

(event EventOnRepCards
  (CallFunction|Rearrange))

(fn ConstructionScript
  (|CallParentFunction))

(fn GetCardat
  (params (At :type Integer))
  (bind _output_get (LocalVariables|SetChosenOne (Utilities|Array|Get(acopy) (Variables|Default|GetCards) At)))
  (Transformation|DetachFromActor _output_get "KeepWorld" "KeepWorld" "KeepRelative")
  (Utilities|Array|RemoveIndex (Variables|Default|GetCards) At)
  (CallFunction|Rearrange)
  (return (LocalVariables|GetChosenOne)))

(fn CheckCardat
  (params (At :type Integer))
  (return (Utilities|Array|Get(acopy) (Variables|Default|GetCards) At)))