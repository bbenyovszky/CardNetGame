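; Game mode for Lard, a trick-taking card game, handling player joins, dealing, hits and scoring.
; It sorts level decks into draw, put, gather and hand roles by name prefix, seats players at tagged starts and starts play when full.
; Played cards hit by matching the put pile's first rank or a wild rank.
; New rounds refill hands to four as supply allows and give the last hitter the pile, scoring two specific ranks.
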(event Custom|FillHands
  (bind _drawdeck (Variables|Default|GetDrawDeck))
  (bind _numofcards (Default|NumOfCards _drawdeck))
  (bind _returnvalue (/ _numofcards 2))
  (for _array_element (Variables|Default|GetHands)
    (bind _cards (Default|GetCards (Variables|Default|GetDrawDeck) (Math|Integer|SelectInt (- 4 (Default|NumOfCards _array_element)) _returnvalue (< (- 4 (Default|NumOfCards _array_element)) _returnvalue)) false))
    (Default|AddCards _array_element _cards true)))

(event Custom|EndRound
  (bind _returnvalue (Game|GetGameState))
  (bind _allplayercontrollers (Variables|Default|GetAllPlayerControllers))
  (bind _aslard_gs (Utilities|Casting|CastToLardGS _returnvalue))
  (bind _currentplayer (Default|CurrentPlayer _aslard_gs))
  (bind _item (Utilities|Array|Get(acopy) _allplayercontrollers _currentplayer))
  (if (Math|Boolean|ORBoolean (== 0 (Default|NumOfCards (Utilities|Array|Get(acopy) (Variables|Default|GetHands) _currentplayer))) (== _currentplayer (Variables|Default|GetLastHit)) (not (Default|CanHit (.AsLard%20PS (Utilities|Casting|CastToLardPS (Variables|/Script/Engine.Controller|GetPlayerState _item))))))
    (CallFunction|NewRound)
    (else
      (Default|SetPass _item true))))

(event Custom|PassRound
  (CallFunction|NewRound))

(event Custom|NewRound
  (bind _lasthit (Variables|Default|GetLastHit))
  (CallFunction|FillHands)
  (CallFunction|PutDecktoPlayer _lasthit)
  (Default|NewRound (.AsLard%20GS (Utilities|Casting|CastToLardGS (Game|GetGameState))) _lasthit))

(event Custom|PutDeckToPlayer
  (params (To :type Integer))
  (bind _putdeck (Variables|Default|GetPutDeck))
  (bind _allplayercontrollers (Variables|Default|GetAllPlayerControllers))
  (bind _item (Utilities|Array|Get(acopy) _allplayercontrollers To))
  (bind _playerstate (Variables|/Script/Engine.Controller|GetPlayerState _item))
  (bind _aslard_ps (Utilities|Casting|CastToLardPS _playerstate))
  (bind _cards (Default|GetCards _putdeck (Default|NumOfCards _putdeck) false))
  (Default|AddCards (Utilities|Array|Get(acopy) (Variables|Default|GetGatherDecks) To) _cards true)
  (for _array_element _cards
    (if (or (Utilities|Enum|Equal(Enum) (Default|GetRank _array_element) "NewEnumerator10") (Utilities|Enum|Equal(Enum) (Default|GetRank _array_element) "NewEnumerator1"))
      (Variables|/Game/Blueprints/Lard/LardPS.LardPS_C|SetPoints _aslard_ps (+ 1 (Variables|/Game/Blueprints/Lard/LardPS.LardPS_C|GetPoints _aslard_ps))))))

(event Custom|PassCard
  (params (CardNumber :type Integer))
  (bind _returnvalue (Game|GetGameState))
  (bind _putdeck (Variables|Default|GetPutDeck))
  (bind _aslard_gs (Utilities|Casting|CastToLardGS _returnvalue))
  (bind _card (Default|GetCardat (Utilities|Array|Get(acopy) (Variables|Default|GetHands) (Default|CurrentPlayer _aslard_gs)) CardNumber))
  (Default|AddCard _putdeck _card true)
  (if (<= (Default|NumOfCards _putdeck) 1)
    (Variables|Default|SetBaseRank (Default|GetRank _card))
    (elif (CallFunction|IsHitCard _card)
      (Variables|Default|SetLastHit (Default|CurrentPlayer (.AsLard%20GS (Utilities|Casting|CastToLardGS (Game|GetGameState)))))))
  (Default|NextPlayer _aslard_gs))

(event Custom|RefreshPoints
  (for _array_element (Variables|Default|GetAllPlayerControllers)
    (Default|RefreshPoints _array_element)))

(event EventPostLogin
  (params (NewPlayer :type Player%20Controller%20Object%20Reference))
  (bind _aslard_pc (Utilities|Casting|CastToLardPC NewPlayer))
  (bind _returnvalue (Pawn|GetControlledPawn _aslard_pc))
  (Utilities|FlowControl|Sequence
    (:then_0
      (Networking|SwitchHasAuthority
        (:Authority
          (bind _returnvalue_2 (Utilities|Array|Add (Variables|Default|GetAllPlayerControllers) _aslard_pc))
          (bind _playerstart (CallFunction|GetPlayerStart _returnvalue_2))
          (Utilities|IsValid _returnvalue
            (:Is%20Valid
              (Transformation|SetActorTransform _returnvalue (Transformation|GetActorTransform _playerstart) false true))
            (:Is%20Not%20Valid
              (bind _returnvalue_3 (Game|SpawnActorfromClass (Variables|Default|GetDefaultPawnClass) (Transformation|GetActorTransform _playerstart) "Undefined" 0 0))
              (Pawn|Possess _aslard_pc _returnvalue_3)))
          (Default|InitialSetup _aslard_pc _returnvalue_2)
          (Development|PrintString (Utilities|String|Append (Variables|/Script/Engine.PlayerState|GetPlayerName (Variables|/Script/Engine.Controller|GetPlayerState _aslard_pc)) " joined the game!") true true "(R=0.000000,G=1.000000,B=0.000000,A=1.000000)" 6.0))))
    (:then_1
      (if (== (Utilities|Array|Length (Variables|Default|GetAllPlayerControllers)) (Variables|Default|GetMaxPlayers))
        (CallFunction|NewRound)
        (CallFunction|RefreshPoints)))))

(event EventBeginPlay
  (bind _outactors (Actor|GetAllActorsOfClass "/Game/Blueprints/AllLevels/DeckBP.DeckBP_C"))
  (for _array_element _outactors
    (switch string (Utilities|String|Left (Utilities|GetDisplayName _array_element) 1)
      (:D
        (bind _output_get (Variables|Default|SetDrawDeck _array_element))
        (Default|GermanSuit _output_get "NewEnumerator0" true))
      (:P
        (Variables|Default|SetPutDeck _array_element))
      (:G
        (Utilities|Array|SetArrayElem (Variables|Default|GetGatherDecks) (Math|Conversions|ToInteger(Byte) (Utilities|String|Right (Utilities|GetDisplayName _array_element) 1)) _array_element))
      (:H
        (Utilities|Array|SetArrayElem (Variables|Default|GetHands) (Math|Conversions|ToInteger(Byte) (Utilities|String|Right (Utilities|GetDisplayName _array_element) 1)) (.AsHand%20Deck%20BP (Utilities|Casting|CastToHandDeckBP _array_element)))))))

(fn ConstructionScript
  (bind _outactors (Actor|GetAllActorsOfClass "/Game/Blueprints/AllLevels/DeckBP.DeckBP_C"))
  (for _array_element _outactors
    (switch string (Utilities|String|Left (Utilities|GetObjectName _array_element) 1)
      (:D
        (Variables|Default|SetDrawDeck _array_element))
      (:P
        (Variables|Default|SetPutDeck _array_element)))))

(fn GetPlayerStart
  (params (Player :type Integer))
  (bind _outactors (Actor|GetAllActorsOfClass "/Script/Engine.PlayerStart"))
  (bind _array_element (Utilities|Array|ForEachLoopwithBreak _outactors :!label _label)
    (:LoopBody
      (if (Utilities|Name|Equal(Name) (Variables|/Script/Engine.PlayerStart|GetPlayerStartTag _array_element) (Utilities|String|StringToName (Utilities|String|ToString(Text) (Utilities|Text|FormatText "Player{Number}Start" Player))))
        (goto _label Break)))
    (:Completed
      (return _array_element))))

(fn IsHitCard
  (params (Card :type Card%20BP%20Object%20Reference))
  (bind _rank (Default|GetRank Card))
  (return (or (Utilities|Enum|Equal(Enum) _rank (Default|GetRank (Utilities|Array|Get(acopy) (Variables|/Game/Blueprints/AllLevels/DeckBP.DeckBP_C|GetCards (Variables|Default|GetPutDeck))))) (Utilities|Enum|Equal(Enum) _rank "NewEnumerator7"))))