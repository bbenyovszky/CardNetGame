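; LardGS, apparently the game state for the Lard game, tracks turn order within rounds.
; It caches the player count from LardGM at BeginPlay, and NewRound sets the starting player and resets a relative turn counter.
; CurrentPlayer derives the active index from starter plus counter, wrapped by player count.
; NextPlayer increments the counter, calls EndRound on LardGM when it reaches a multiple of that count, and returns the current player.
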(event Custom|NewRound
  (params (StartPlayer :type Integer))
  (Variables|Default|SetRoundStarter StartPlayer)
  (Variables|Default|SetRelativePlayer 0))

(event EventBeginPlay
  (Variables|Default|SetMaxPlayer (Variables|/Game/Blueprints/Lard/LardGM.LardGM_C|GetMaxPlayers (.AsLard%20GM (Utilities|Casting|CastToLardGM (Game|GetGameMode))))))

(fn ConstructionScript)

(fn NextPlayer
  (bind _result (Math|Integer|IncrementInt (Variables|Default|GetRelativePlayer))
    (:%20%20
      (if (!= (Math|Integer|%(Integer) _result (Variables|Default|GetMaxPlayer)) 0)
        _
        (else
          (Default|EndRound (.AsLard%20GM (Utilities|Casting|CastToLardGM (Game|GetGameMode))))))
      (return (CallFunction|CurrentPlayer)))))

(fn CurrentPlayer
  (return (Math|Integer|%(Integer) (+ (Variables|Default|GetRoundStarter) (Variables|Default|GetRelativePlayer)) (Variables|Default|GetMaxPlayer))))