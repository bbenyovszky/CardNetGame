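; LardPC is the player controller for the Lard game mode, linking each player to the LardWB on-screen widget.
; ClientSetup runs the parent setup, then creates the widget for this controller and adds it to the viewport.
; SetPass writes the CanPass flag to the LardPS player state and passes it to the widget.
; RefreshPoints forwards point refresh requests to the widget.
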(event Custom|SetPass
  (params (Can :type Boolean))
  (Variables|/Game/Blueprints/Lard/LardPS.LardPS_C|SetCanPass (.AsLard%20PS (Utilities|Casting|CastToLardPS (Variables|Default|GetPlayerState))) Can)
  (Default|CanPass (Variables|Default|GetLardWB) Can))

(event Custom|RefreshPoints
  (Default|RefreshPoints (Variables|Default|GetLardWB)))

(event EventClientSetup
  (params (PlayerNumber :type Integer))
  (|CallParentFunction PlayerNumber)
  (bind _returnvalue (UserInterface|CreateWidget "/Game/UI/Lard/LardWB.LardWB_C" self))
  (bind _output_get (Variables|Default|SetLardWB _returnvalue))
  (UserInterface|Viewport|AddtoViewport _output_get 0))

(fn ConstructionScript)