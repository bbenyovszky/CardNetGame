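; LardPS is the player state for the Lard card game, binding a player to a hand deck and validating that player's moves.
; Setup matches a HandDeckBP by the last digit of its display name.
; Clicked cards reach LardGM only on that player's turn, restricted to the base rank or one fixed wild rank while passing is allowed.
; CanHit checks for such cards, and replicated points refresh LardPC's display.
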(event Custom|PassRound
  (Variables|Default|SetCanPass false)
  (Default|PassRound (.AsLard%20GM (Utilities|Casting|CastToLardGM (Game|GetGameMode)))))

(event EventInitialSetup
  (params (PlayerNumber :type Integer))
  (|CallParentFunction PlayerNumber)
  (bind _outactors (Actor|GetAllActorsOfClass "/Game/Blueprints/AllLevels/HandDeckBP.HandDeckBP_C"))
  (bind _array_element (Utilities|Array|ForEachLoopwithBreak _outactors :!label _label)
    (:LoopBody
      (if (== (Math|Conversions|ToInteger(Byte) (Utilities|String|Right (Utilities|GetDisplayName _array_element) 1)) (Variables|Default|GetMyNumber))
        (goto _label Break)))
    (:Completed
      (Variables|Default|SetHandDeck _array_element))))

(event EventCardClicked
  (params (ClickedCard :type Card%20BP%20Object%20Reference) (LeftClick :type Boolean))
  (bind _rank (Default|GetRank ClickedCard))
  (bind _handdeck (Variables|Default|GetHandDeck))
  (bind _number (Default|ContainsThis _handdeck ClickedCard))
  (if (Math|Boolean|ANDBoolean (!= _number -1) (== (Default|CurrentPlayer (.AsLard%20GS (Utilities|Casting|CastToLardGS (Game|GetGameState)))) (Variables|Default|GetMyNumber)) (or (or (Utilities|Enum|Equal(Enum) "NewEnumerator7" _rank) (Utilities|Enum|Equal(Enum) _rank (Variables|/Game/Blueprints/Lard/LardGM.LardGM_C|GetBaseRank (.AsLard%20GM (Utilities|Casting|CastToLardGM (Game|GetGameMode)))))) (not (Variables|Default|GetCanPass))))
    (if (Variables|Default|GetCanPass)
      (Default|SetPass (.AsLard%20PC (Utilities|Casting|CastToLardPC (Components|GetOwner))) false))
    (Default|PassCard (.AsLard%20GM (Utilities|Casting|CastToLardGM (Game|GetGameMode))) _number)))

(fn ConstructionScript
  (|CallParentFunction))

(fn CanHit
  (bind _array_element (Utilities|Array|ForEachLoopwithBreak (Variables|/Game/Blueprints/AllLevels/DeckBP.DeckBP_C|GetCards (Variables|Default|GetHandDeck)) :!label _label)
    (:LoopBody
      (if (or (Utilities|Enum|Equal(Enum) "NewEnumerator7" (Default|GetRank _array_element)) (Utilities|Enum|Equal(Enum) (Default|GetRank _array_element) (Variables|/Game/Blueprints/Lard/LardGM.LardGM_C|GetBaseRank (.AsLard%20GM (Utilities|Casting|CastToLardGM (Game|GetGameMode))))))
        (goto _label Break)))
    (:Completed
      (return (or (Utilities|Enum|Equal(Enum) "NewEnumerator7" (Default|GetRank _array_element)) (Utilities|Enum|Equal(Enum) (Default|GetRank _array_element) (Variables|/Game/Blueprints/Lard/LardGM.LardGM_C|GetBaseRank (.AsLard%20GM (Utilities|Casting|CastToLardGM (Game|GetGameMode))))))))))

(fn OnRepPoints
  (Default|RefreshPoints (.AsLard%20PC (Utilities|Casting|CastToLardPC (Game|GetPlayerController 0)))))