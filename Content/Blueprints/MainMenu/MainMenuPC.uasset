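; Main menu player controller that switches between the main, new game and options menus and handles online matchmaking.
; Each menu swaps in a cached widget while a timeline lerps the menu camera to that menu's spot actor, both found by name at startup.
; JoinGame searches sessions filtered by GameType and joins the first non-full one, otherwise hosts a listen server on that type's map.
; An older matchmaking version remains unconnected.
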(event Custom|ShowMainMenu
  ;[1 1 1] Show the Main Menu
  (Utilities|IsValid (Variables|Default|GetMainMenuWB)
    (:Is%20Valid
      _)
    (:Is%20Not%20Valid
      (bind _returnvalue (UserInterface|CreateWidget "/Game/UI/MainMenu/MainMenu.MainMenu_C"))
      (bind _output_get (Variables|Default|SetMainMenuWB _returnvalue))))
  (Viewport|RemoveAllWidgets)
  (UserInterface|Viewport|AddtoViewport _output_get 0)
  (CallFunction|MoveCamerato (Transformation|GetActorTransform (Variables|Default|GetMenuCamera)) (Variables|Default|GetMainMenuSpot)))

(event Custom|JoinGame
  (params (GameType :type EGameType%20Enum))
  (bind _returnvalue (Class|KismetSystemLibrary|MakeLiteralInteger 13000))
  (bind _returnvalue_2 (Class|AdvancedSessionsLibrary|MakeLiteralSessionPropertyByte "GameType" GameType))
  (bind _self self)
  (Development|PrintText (Utilities|Text|FormatText "Starting search through {Number} servers..." _returnvalue) true true "(R=0.000000,G=0.660000,B=1.000000,A=1.000000)" 6.0)
  (bind _results (|FindSessions self _returnvalue false)
    (:OnSuccess
      (Development|PrintText (Utilities|Text|FormatText "Found {Num} servers." (Utilities|Array|Length _results)) true true "(R=0.000000,G=1.000000,B=0.000000,A=1.000000)" 6.0)
      (bind _filteredresults (Class|FindSessionsCallbackProxyAdvanced|FilterSessionResults _results (Utilities|Array|MakeArray (Class|AdvancedSessionsLibrary|MakeLiteralSessionSearchProperty _returnvalue_2 "Equals"))))
      (Development|PrintText (Utilities|Text|FormatText "Filtered to {Num} servers." (Utilities|Array|Length _filteredresults)) true true "(R=0.000000,G=1.000000,B=0.000000,A=1.000000)" 6.0)
      (Variables|Default|SetFoundSession? false)
      (bind _array_element (Utilities|Array|ForEachLoopwithBreak _filteredresults :!label _label)
        (:LoopBody
          (Development|PrintText (Utilities|Text|FormatText "Server: {Server} - {Current}/{Max} - Join: {bool}" (Utilities|Text|ToText(String) (Class|FindSessionsCallbackProxy|GetServerName _array_element)) (Class|FindSessionsCallbackProxy|GetCurrentPlayers _array_element) (Class|FindSessionsCallbackProxy|GetMaxPlayers _array_element) (Utilities|Text|ToText(Boolean) (not (== (Class|FindSessionsCallbackProxy|GetCurrentPlayers _array_element) (Class|FindSessionsCallbackProxy|GetMaxPlayers _array_element))))) true true "(R=1.000000,G=0.975130,B=0.000000,A=1.000000)" 1e+01)
          (if (not (== (Class|FindSessionsCallbackProxy|GetCurrentPlayers _array_element) (Class|FindSessionsCallbackProxy|GetMaxPlayers _array_element)))
            (Variables|Default|SetFoundSession? true)
            (goto _label Break)))
        (:Completed
          (if (Variables|Default|GetFoundSession?)
            (Development|PrintText (Utilities|Text|FormatText "Joining to {Name} server." (Utilities|Text|ToText(String) (Class|FindSessionsCallbackProxy|GetServerName _array_element))) true true "(R=0.000000,G=1.000000,B=0.000000,A=1.000000)" 6.0)
            (|JoinSession _self _array_element
              (:OnFailure
                (Development|PrintText "Failed to join session." true true "(R=1.000000,G=0.000000,B=0.000000,A=1.000000)" 6.0)))
            (else
              (Development|PrintText "Server was not valid." true true "(R=1.000000,G=0.000000,B=0.000000,A=1.000000)" 6.0)))
          (|AdvancedSession (Utilities|Array|MakeArray _returnvalue_2) _self 2 0 false true false true true false false false true :!label _label_2
            (:OnSuccess
              (Game|OpenLevel(byName) (Utilities|String|StringToName (Utilities|String|Append (Utilities|String|EnumtoString GameType) "Map")) true "listen"))
            (:OnFailure
              (Development|PrintText "Failed to create session." true true "(R=1.000000,G=0.000000,B=0.000000,A=1.000000)" 6.0))))))
    (:OnFailure
      (Development|PrintText "Couldn't find servers." true true "(R=1.000000,G=0.000000,B=0.000000,A=1.000000)" 6.0)
      (goto _label_2))))

(event Custom|ShowNewGameMenu
  ;[1 1 1] Show the New Game Menu
  (Utilities|IsValid (Variables|Default|GetNewGameMenuWB)
    (:Is%20Valid
      _)
    (:Is%20Not%20Valid
      (bind _returnvalue (UserInterface|CreateWidget "/Game/UI/MainMenu/NewGameMenu.NewGameMenu_C"))
      (bind _output_get (Variables|Default|SetNewGameMenuWB _returnvalue))))
  (Viewport|RemoveAllWidgets)
  (UserInterface|Viewport|AddtoViewport _output_get 0)
  (CallFunction|MoveCamerato (Transformation|GetActorTransform (Variables|Default|GetMenuCamera)) (Variables|Default|GetNewGameSpot)))

(event Custom|MoveCameraTo
  (params (From :type Transform) (To :type Actor%20Object%20Reference))
  ;[1 1 1] Moves the camera to the given position
  (bind _alpha (Timeline|Timeline_0 PlayFromStart)
    (:Update
      (Transformation|SetActorTransform (Variables|Default|GetMenuCamera) (Math|Transform|Lerp(Transform) From (Transformation|GetActorTransform To) _alpha)))))

(event Custom|ShowOptionsMenu
  ;[1 1 1] Show the Options Menu
  (Utilities|IsValid (Variables|Default|GetOptionsMenuWB)
    (:Is%20Valid
      _)
    (:Is%20Not%20Valid
      (bind _returnvalue (UserInterface|CreateWidget "/Game/UI/MainMenu/OptionsMenu.OptionsMenu_C"))
      (bind _output_get (Variables|Default|SetOptionsMenuWB _returnvalue))))
  (Viewport|RemoveAllWidgets)
  (UserInterface|Viewport|AddtoViewport _output_get 0)
  (CallFunction|MoveCamerato (Transformation|GetActorTransform (Variables|Default|GetMenuCamera)) (Variables|Default|GetOptionsSpot)))

(event EventBeginPlay
  ;[1 1 1] Get the camera and the positions, and show the Main Menu
  (Utilities|FlowControl|Sequence
    (:then_0
      (Input|SetInputModeUIOnly self 0 "DoNotLock"))
    (:then_1
      (bind _outactors (Actor|GetAllActorsOfClass "/Script/Engine.CameraActor"))
      (bind _array_element (Utilities|Array|ForEachLoopwithBreak _outactors :!label _label)
        (:LoopBody
          (if (Utilities|Enum|Equal(Enum) "MainMenuCamera" (Utilities|GetObjectName _array_element))
            (Variables|Default|SetMenuCamera _array_element)
            (goto _label Break)))))
    (:then_2
      (bind _outactors_2 (Actor|GetAllActorsOfClass "/Script/Engine.Actor"))
      (for _array_element_2 _outactors_2
        (switch string (Utilities|GetObjectName _array_element_2)
          (:MainMenuSpot
            (Variables|Default|SetMainMenuSpot _array_element_2))
          (:NewGameSpot
            (Variables|Default|SetNewGameSpot _array_element_2))
          (:OptionsSpot
            (Variables|Default|SetOptionsSpot _array_element_2)))))
    (:then_3
      (CallFunction|ShowMainMenu))))

(fn ConstructionScript)