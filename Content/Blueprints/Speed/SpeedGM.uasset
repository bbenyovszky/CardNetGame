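; Game mode for the two-player card game Speed, seating players at tagged starts and running the match.
; State changes go from waiting through ready to ongoing, mirrored to SpeedGS and each controller's widget.
; When all players ready up, cards are dealt onto both right decks, with fallbacks for empty decks.
; It validates one-rank-away moves, makes the opponent absorb their piles on SPEED, and resets after a win.
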(event Custom|PassCard
  (params (From :type Deck%20BP%20Object%20Reference) (To :type Deck%20BP%20Object%20Reference))
  (bind _card (Default|CheckTopCard From))
  (bind _card_2 (Default|CheckTopCard To))
  (if (Math|Boolean|ANDBoolean (not (Default|Empty From)) (not (Default|Empty To)) (Utilities|Enum|Equal(Enum) (Variables|Default|GetCurrentState) "NewEnumerator2"))
    (if (Default|OneRankAway _card _card_2)
      (bind _card_3 (Default|GetCard From true))
      (Default|AddCard To _card_3 true)
      (CallFunction|ResetReady)
      (else
        (Development|PrintText (Utilities|Text|FormatText "You can't put {This} to {That}" (Utilities|Text|ToText(String) (Utilities|String|EnumtoString (Variables|/Game/Blueprints/AllLevels/CardBP.CardBP_C|GetRank _card))) (Utilities|Text|ToText(String) (Utilities|String|EnumtoString (Variables|/Game/Blueprints/AllLevels/CardBP.CardBP_C|GetRank _card_2)))))))))

(event Custom|14
  (bind _allplayercontrollers (Variables|Default|GetAllPlayerControllers))
  (bind _item (Utilities|Array|Get(acopy) _allplayercontrollers 1))
  (bind _item_2 (Utilities|Array|Get(acopy) _allplayercontrollers))
  (bind _playerstate (Variables|/Script/Engine.Controller|GetPlayerState _item_2))
  (bind _playerstate_2 (Variables|/Script/Engine.Controller|GetPlayerState _item))
  (bind _asspeed_ps (Utilities|Casting|CastToSpeedPS _playerstate_2))
  (bind _asspeed_ps_2 (Utilities|Casting|CastToSpeedPS _playerstate))
  (bind _playerdeck (Default|GetPlayerDeck _asspeed_ps))
  (bind _rightdeck (Default|GetRightDeck _asspeed_ps))
  (bind _playerdeck_2 (Default|GetPlayerDeck _asspeed_ps))
  (bind _playerdeck_3 (Default|GetPlayerDeck _asspeed_ps_2))
  (bind _playerdeck_4 (Default|GetPlayerDeck _asspeed_ps_2))
  (bind _rightdeck_2 (Default|GetRightDeck _asspeed_ps_2))
  (bind _empty (Default|Empty _playerdeck_2))
  (bind _empty_2 (Default|Empty _playerdeck_3))
  (bind _returnvalue (Math|Integer|SelectInt 2 0 _empty))
  (bind _returnvalue_2 (Math|Integer|SelectInt 1 0 _empty_2))
  (bind _returnvalue_3 (+ _returnvalue_2 _returnvalue))
  (bind _returnvalue_4 (!= _returnvalue_3 3))
  (if (Utilities|Enum|NotEqual(Enum) (Variables|Default|GetCurrentState) "NewEnumerator0")
    (Variables|Default|SetSomeoneIsReady true)
    (bind _array_element (Utilities|Array|ForEachLoopwithBreak (Variables|Default|GetAllPlayerControllers) :!label _label)
      (:LoopBody
        (if (not (Variables|/Game/Blueprints/Speed/SpeedPS.SpeedPS_C|GetReady (.AsSpeed%20PS (Utilities|Casting|CastToSpeedPS (Variables|/Script/Engine.Controller|GetPlayerState _array_element)))))
          (goto _label Break)))
      (:Completed
        (if (Variables|/Game/Blueprints/Speed/SpeedPS.SpeedPS_C|GetReady (.AsSpeed%20PS (Utilities|Casting|CastToSpeedPS (Variables|/Script/Engine.Controller|GetPlayerState _array_element))))
          (CallFunction|SetCurrentState "NewEnumerator2")
          (Utilities|FlowControl|Sequence
            (:then_0
              (bind _card (Default|GetCard (Utilities|Select :Index _returnvalue_3 :Option%200 _playerdeck_4 :Option%201 _playerdeck :Option%202 _playerdeck_4 :Option%203 _rightdeck_2) _returnvalue_4))
              (Default|AddCard _rightdeck_2 _card true))
            (:then_1
              (bind _card_2 (Default|GetCard (Utilities|Select :Index _returnvalue_3 :Option%200 _playerdeck :Option%201 _playerdeck :Option%202 _playerdeck_4 :Option%203 _rightdeck) _returnvalue_4))
              (Default|AddCard _rightdeck _card_2 true))
            (:then_2
              (CallFunction|ResetReady))))))))

(event Custom|FillWithOne
  (params (From :type Deck%20BP%20Object%20Reference) (To :type Deck%20BP%20Object%20Reference))
  (if (and (not (Default|Empty From)) (Default|Empty To))
    (bind _card (Default|GetCard From true))
    (Default|AddCard To _card true)))

(event Custom|I%20Won
  (params (Me :type String))
  (Development|PrintText (Utilities|Text|FormatText "{Player} WON!" (Utilities|Text|ToText(String) Me)) true true "(R=0.000000,G=1.000000,B=0.017753,A=1.000000)" 5.0)
  (Utilities|FlowControl|Sequence
    (:then_0
      (bind _outactors (Actor|GetAllActorsOfClass "/Game/Blueprints/AllLevels/DeckBP.DeckBP_C"))
      (for _array_element _outactors
        (Default|Clear _array_element)))
    (:then_1
      (for (_array_element_2 _array_index) (Variables|Default|GetAllPlayerControllers)
        (Default|InitialSetup (.AsGame%20PS (Utilities|Casting|CastToGamePS (Variables|/Script/Engine.Controller|GetPlayerState _array_element_2))) _array_index))
      (CallFunction|SetCurrentState "NewEnumerator1"))))

(event Custom|SPEED
  (params (Me :type Integer))
  (bind _returnvalue (Utilities|Select :Index Me :Option%200 1 :Option%201 0))
  (bind _allplayercontrollers (Variables|Default|GetAllPlayerControllers))
  (bind _item (Utilities|Array|Get(acopy) _allplayercontrollers _returnvalue))
  (bind _playerstate (Variables|/Script/Engine.Controller|GetPlayerState _item))
  (bind _asspeed_ps (Utilities|Casting|CastToSpeedPS _playerstate))
  (bind _playerdeck (Default|GetPlayerDeck _asspeed_ps))
  (for _index (range 0 1)
    (while (not (Default|Empty (Utilities|Select :Index _index :Option%200 (Default|GetLeftDeck _asspeed_ps) :Option%201 (Default|GetRightDeck _asspeed_ps))))
      (bind _card (Default|GetCard (Utilities|Select :Index _index :Option%200 (Default|GetLeftDeck _asspeed_ps) :Option%201 (Default|GetRightDeck _asspeed_ps)) false))
      (Default|AddCard _playerdeck _card true)))
  (Default|Shuffle _playerdeck)
  (Default|Rearrange _playerdeck)
  (Default|FillSpots _asspeed_ps)
  (CallFunction|SetCurrentState "NewEnumerator1"))

(event EventPostLogin
  (params (NewPlayer :type Player%20Controller%20Object%20Reference))
  (bind _asspeed_pc (Utilities|Casting|CastToSpeedPC NewPlayer))
  (bind _returnvalue (Pawn|GetControlledPawn _asspeed_pc))
  (Utilities|FlowControl|Sequence
    (:then_0
      (Networking|SwitchHasAuthority
        (:Authority
          (bind _returnvalue_2 (Utilities|Array|Add (Variables|Default|GetAllPlayerControllers) _asspeed_pc))
          (bind _playerstart (CallFunction|GetPlayerStart _returnvalue_2))
          (Utilities|IsValid _returnvalue
            (:Is%20Valid
              (Transformation|SetActorTransform _returnvalue (Transformation|GetActorTransform _playerstart) false true))
            (:Is%20Not%20Valid
              (bind _returnvalue_3 (Game|SpawnActorfromClass (Variables|Default|GetDefaultPawnClass) (Transformation|GetActorTransform _playerstart) "Undefined" 0 0))
              (Pawn|Possess _asspeed_pc _returnvalue_3)))
          (Default|InitialSetup _asspeed_pc _returnvalue_2)
          (for _array_element (Variables|Default|GetAllPlayerControllers)
            (Default|UpdateSpeedWidget _array_element "NewEnumerator0"))
          (Development|PrintText (Utilities|Text|FormatText "{Player} joined the game!" (Utilities|Text|ToText(String) (Variables|/Script/Engine.PlayerState|GetPlayerName (Variables|/Script/Engine.Controller|GetPlayerState _asspeed_pc)))) true true "(R=0.000000,G=1.000000,B=0.017753,A=1.000000)" 5.0))))
    (:then_1
      (if (== (Utilities|Array|Length (Variables|Default|GetAllPlayerControllers)) (Variables|Default|GetMaxPlayers))
        (CallFunction|SetCurrentState "NewEnumerator1")))))

(fn ConstructionScript)

(fn GetPlayerStart
  (params (Player :type Integer))
  (bind _outactors (Actor|GetAllActorsOfClass "/Script/Engine.PlayerStart"))
  (bind _array_element (Utilities|Array|ForEachLoopwithBreak _outactors :!label _label)
    (:LoopBody
      (if (Utilities|Name|Equal(Name) (Variables|/Script/Engine.PlayerStart|GetPlayerStartTag _array_element) (Utilities|Select :Index Player :Option%200 "Player0Start" :Option%201 "Player1Start"))
        (goto _label Break)))
    (:Completed
      (return _array_element))))

(fn SetCurrentState
  (params (NewState :type SpeedState%20Enum))
  (Development|PrintString (Utilities|String|EnumtoString NewState) true true "(R=1.000000,G=0.896179,B=0.000000,A=1.000000)" 6.0)
  (for _array_element (Variables|Default|GetAllPlayerControllers)
    (Default|UpdateSpeedWidget _array_element NewState))
  (bind _output_get (Variables|Default|SetCurrentState NewState))
  (Variables|/Game/Blueprints/Speed/SpeedGS.SpeedGS_C|SetCurrentState (.AsSpeed%20GS (Utilities|Casting|CastToSpeedGS (Game|GetGameState))) _output_get)
  (switch Utilities|FlowControl|Switch|SwitchonSpeedState _output_get
    (:NewEnumerator0
      _)
    (:NewEnumerator1
      _)
    (:NewEnumerator2
      _))
  (return NewState))

(fn GetCurrentState
  (return (Variables|Default|GetCurrentState)))

(fn ResetReady
  (if (Variables|Default|GetSomeoneIsReady)
    (Variables|Default|SetSomeoneIsReady false)
    (for _array_element (Variables|Default|GetAllPlayerControllers)
      (Variables|/Game/Blueprints/Speed/SpeedPS.SpeedPS_C|SetReady (.AsSpeed%20PS (Utilities|Casting|CastToSpeedPS (Variables|/Script/Engine.Controller|GetPlayerState _array_element))) false))))