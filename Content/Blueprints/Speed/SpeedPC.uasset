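; Player controller for the Speed card game, turning key and mouse wheel input into player actions and creating and updating the on-screen SpeedWB widget.
; Held keys fill source (A/S/D/F/G) and target (Left/Right) arrays; one of each triggers PassCard on SpeedPS with zero-based indices.
; Wheel up or Up calls SpeedGuess, wheel down or Space calls SpeedPS function "14", and W reports a win to SpeedGM.
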(event Custom|UpdateSpeedWidget
  (params (CurrentState :type SpeedState%20Enum))
  (Utilities|IsValid (Variables|Default|GetSpeedWB)
    (:Is%20Valid
      _)
    (:Is%20Not%20Valid
      (bind _returnvalue (UserInterface|CreateWidget "/Game/UI/Speed/SpeedWB.SpeedWB_C"))
      (bind _output_get (Variables|Default|SetSpeedWB _returnvalue))
      (UserInterface|Viewport|AddtoViewport _output_get 0)))
  (Default|Update _output_get CurrentState))

(event Custom|wining
  (Default|IWon (.AsSpeed%20GM (Utilities|Casting|CastToSpeedGM (Game|GetGameMode))) "Reset"))

(event Input|KeyboardEvents|A
  (params (Key :type Key%20Structure :default "AnyKey"))
  (bind _returnvalue (Class|KismetSystemLibrary|MakeLiteralInteger 3))
  (:Pressed
    (CallFunction|SetCardButtons true _returnvalue))
  (:Released
    (CallFunction|SetCardButtons false _returnvalue)))

(event Input|KeyboardEvents|Left
  (params (Key :type Key%20Structure :default "AnyKey"))
  (bind _returnvalue (Class|KismetSystemLibrary|MakeLiteralInteger 1))
  (:Pressed
    (CallFunction|SetCardButtons true _returnvalue))
  (:Released
    (CallFunction|SetCardButtons false _returnvalue)))

(event Input|KeyboardEvents|Right
  (params (Key :type Key%20Structure :default "AnyKey"))
  (bind _returnvalue (Class|KismetSystemLibrary|MakeLiteralInteger 2))
  (:Pressed
    (CallFunction|SetCardButtons true _returnvalue))
  (:Released
    (CallFunction|SetCardButtons false _returnvalue)))

(event Input|KeyboardEvents|G
  (params (Key :type Key%20Structure :default "AnyKey"))
  (bind _returnvalue (Class|KismetSystemLibrary|MakeLiteralInteger 7))
  (:Pressed
    (CallFunction|SetCardButtons true _returnvalue))
  (:Released
    (CallFunction|SetCardButtons false _returnvalue)))

(event Input|MouseEvents|MouseWheelUp
  (params (Key :type Key%20Structure :default "AnyKey"))
  (:Pressed
    (Default|SpeedGuess (.AsSpeed%20PS (Utilities|Casting|CastToSpeedPS (Variables|Default|GetPlayerState))))))

(event Input|MouseEvents|MouseWheelDown
  (params (Key :type Key%20Structure :default "AnyKey"))
  (:Pressed
    (Default|14 (.AsSpeed%20PS (Utilities|Casting|CastToSpeedPS (Variables|Default|GetPlayerState))))))

(event Input|KeyboardEvents|SpaceBar
  (params (Key :type Key%20Structure :default "AnyKey"))
  (:Pressed
    (Default|14 (.AsSpeed%20PS (Utilities|Casting|CastToSpeedPS (Variables|Default|GetPlayerState))))))

(event Input|KeyboardEvents|S
  (params (Key :type Key%20Structure :default "AnyKey"))
  (bind _returnvalue (Class|KismetSystemLibrary|MakeLiteralInteger 4))
  (:Pressed
    (CallFunction|SetCardButtons true _returnvalue))
  (:Released
    (CallFunction|SetCardButtons false _returnvalue)))

(event Input|KeyboardEvents|Up
  (params (Key :type Key%20Structure :default "AnyKey"))
  (:Pressed
    (Default|SpeedGuess (.AsSpeed%20PS (Utilities|Casting|CastToSpeedPS (Variables|Default|GetPlayerState))))))

(event Input|KeyboardEvents|D
  (params (Key :type Key%20Structure :default "AnyKey"))
  (bind _returnvalue (Class|KismetSystemLibrary|MakeLiteralInteger 5))
  (:Pressed
    (CallFunction|SetCardButtons true _returnvalue))
  (:Released
    (CallFunction|SetCardButtons false _returnvalue)))

(event Input|KeyboardEvents|W
  (params (Key :type Key%20Structure :default "AnyKey"))
  (:Pressed
    (CallFunction|Wining)))

(event Input|KeyboardEvents|F
  (params (Key :type Key%20Structure :default "AnyKey"))
  (bind _returnvalue (Class|KismetSystemLibrary|MakeLiteralInteger 6))
  (:Pressed
    (CallFunction|SetCardButtons true _returnvalue))
  (:Released
    (CallFunction|SetCardButtons false _returnvalue)))

(fn ConstructionScript)

(fn SetCardButtons
  (params (Add :type Boolean) (Button :type Integer))
  (bind _returnvalue (< Button 3))
  (bind _frombuttons (Variables|Default|GetFromButtons))
  (bind _tobuttons (Variables|Default|GetToButtons))
  (bind _frombuttons_2 (Variables|Default|GetFromButtons))
  (bind _tobuttons_2 (Variables|Default|GetToButtons))
  (bind _returnvalue_2 (select _returnvalue _tobuttons _frombuttons))
  (if Add
    (Utilities|Array|Add _returnvalue_2 Button)
    (else
      (Utilities|Array|RemoveItem _returnvalue_2 Button)))
  (if (and (== (Utilities|Array|Length _frombuttons_2) 1) (== (Utilities|Array|Length _tobuttons_2) 1))
    (Default|PassCard (.AsSpeed%20PS (Utilities|Casting|CastToSpeedPS (Variables|Default|GetPlayerState))) (- (Utilities|Array|Get(acopy) _frombuttons_2) 3) (- (Utilities|Array|Get(acopy) _tobuttons_2) 1))))