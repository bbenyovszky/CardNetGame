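; Player state for the card game Speed, holding one player's deck, five card slots and references to both center piles.
; InitialSetup finds these DeckBP actors by parsing object names, builds a shuffled deck and fills the slots.
; Left or right clicks play cards to either pile through SpeedGM, refilling the slot and checking for a win.
; New-card requests and matching-rank SPEED calls also go to SpeedGM.
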(event Custom|PassCard
  (params (From :type Integer) (To :type Integer))
  (bind _returnvalue (Game|GetGameMode))
  (bind _card0 (Variables|Decks|GetCard0))
  (bind _card1 (Variables|Decks|GetCard1))
  (bind _card2 (Variables|Decks|GetCard2))
  (bind _card3 (Variables|Decks|GetCard3))
  (bind _card4 (Variables|Decks|GetCard4))
  (bind _asspeed_gm (Utilities|Casting|CastToSpeedGM _returnvalue))
  (bind _returnvalue_2 (Utilities|Select :Index From :Option%200 _card0 :Option%201 _card1 :Option%202 _card2 :Option%203 _card3 :Option%204 _card4))
  (Utilities|FlowControl|Sequence
    (:then_0
      (Default|PassCard _asspeed_gm _returnvalue_2 (Utilities|Select :Index To :Option%200 (Variables|Decks|GetLeftDeck) :Option%201 (Variables|Decks|GetRightDeck)))
      (Default|FillwithOne _asspeed_gm (Variables|Decks|GetPlayerDeck) _returnvalue_2))
    (:then_1
      (if (CallFunction|DidIWin)
        (Default|IWon (.AsSpeed%20GM (Utilities|Casting|CastToSpeedGM (Game|GetGameMode))) (Variables|Default|GetPlayerName))))))

(event Custom|FillSpots
  (for _index (range 0 4)
    (Default|FillwithOne (.AsSpeed%20GM (Utilities|Casting|CastToSpeedGM (Game|GetGameMode))) (Variables|Decks|GetPlayerDeck) (Utilities|Select :Index _index :Option%200 (Variables|Decks|GetCard0) :Option%201 (Variables|Decks|GetCard1) :Option%202 (Variables|Decks|GetCard2) :Option%203 (Variables|Decks|GetCard3) :Option%204 (Variables|Decks|GetCard4)))))

(event Custom|14
  (bind _returnvalue (Game|GetGameMode))
  (bind _asspeed_gm (Utilities|Casting|CastToSpeedGM _returnvalue))
  (if (Utilities|Enum|NotEqual(Enum) (Default|GetCurrentState _asspeed_gm) "NewEnumerator0")
    (Variables|Default|SetReady true)
    (Default|14 _asspeed_gm)
    (Development|PrintText (Utilities|Text|FormatText "Player {Number} wants new card!" (Variables|Default|GetMyNumber)) true false "(R=0.000000,G=0.660000,B=1.000000,A=1.000000)" 5.0)))

(event Custom|SpeedGuess
  (bind _returnvalue (Game|GetGameMode))
  (bind _leftdeck (Variables|Decks|GetLeftDeck))
  (bind _rightdeck (Variables|Decks|GetRightDeck))
  (bind _mynumber (Variables|Default|GetMyNumber))
  (bind _asspeed_gm (Utilities|Casting|CastToSpeedGM _returnvalue))
  (if (not (Math|Boolean|ORBoolean (Default|Empty _leftdeck) (Default|Empty _rightdeck) (Utilities|Enum|Equal(Enum) (Default|GetCurrentState _asspeed_gm) "NewEnumerator0")))
    (if (Utilities|Enum|Equal(Enum) (Variables|/Game/Blueprints/AllLevels/CardBP.CardBP_C|GetRank (Default|CheckTopCard _leftdeck)) (Variables|/Game/Blueprints/AllLevels/CardBP.CardBP_C|GetRank (Default|CheckTopCard _rightdeck)))
      (Default|SPEED _asspeed_gm _mynumber)
      (Development|PrintText (Utilities|Text|FormatText "Player {Number}: SPEED!" _mynumber) true true "(R=0.048672,G=1.000000,B=0.000000,A=1.000000)" 5.0))))

(event EventCardClicked
  (params (ClickedCard :type Card%20BP%20Object%20Reference) (LeftClick :type Boolean))
  (bind _defaultsceneroot (Variables|/Game/Blueprints/AllLevels/CardBP.CardBP_C|GetDefaultSceneRoot ClickedCard))
  (bind _returnvalue (Transformation|GetAttachParent _defaultsceneroot))
  (bind _returnvalue_2 (Components|GetOwner _returnvalue))
  (bind _returnvalue_3 (Utilities|GetObjectName _returnvalue_2))
  (if (Utilities|String|StartsWith _returnvalue_3 (Utilities|String|Append "P" (Utilities|String|ToString(Integer) (Variables|Default|GetMyNumber)) "Card"))
    (CallFunction|PassCard (Math|Conversions|ToInteger(Byte) (Utilities|String|Right _returnvalue_3 1)) (Math|Conversions|ToInteger(Boolean) (not LeftClick)))))

(event EventInitialSetup
  (params (PlayerNumber :type Integer))
  (|CallParentFunction PlayerNumber)
  (bind _outactors (Actor|GetAllActorsOfClass "/Game/Blueprints/AllLevels/DeckBP.DeckBP_C"))
  (for _array_element _outactors
    (switch string (Utilities|String|Left (Utilities|GetObjectName _array_element) 1)
      (:C
        (if (Utilities|Enum|Equal(Enum) (Utilities|String|GetSubstring (Utilities|GetObjectName _array_element) 1) (Utilities|String|ToString(Integer) (Variables|Default|GetMyNumber)))
          (Variables|Decks|SetRightDeck _array_element)
          (else
            (Variables|Decks|SetLeftDeck _array_element))))
      (:P
        (if (Utilities|Enum|Equal(Enum) (Utilities|String|GetSubstring (Utilities|GetObjectName _array_element) 1) (Utilities|String|ToString(Integer) (Variables|Default|GetMyNumber)))
          (switch string (Utilities|String|RightChop (Utilities|GetObjectName _array_element) 2)
            (:Card0
              (Variables|Decks|SetCard0 _array_element))
            (:Card1
              (Variables|Decks|SetCard1 _array_element))
            (:Card2
              (Variables|Decks|SetCard2 _array_element))
            (:Card3
              (Variables|Decks|SetCard3 _array_element))
            (:Card4
              (Variables|Decks|SetCard4 _array_element))
            (:Deck
              (bind _output_get (Variables|Decks|SetPlayerDeck _array_element))
              (Default|StandardDeck _output_get (Utilities|Array|MakeArray "NewEnumerator0") false true)))))))
  (CallFunction|FillSpots))

(fn ConstructionScript)

(fn GetPlayerDeck
  (return (Variables|Decks|GetPlayerDeck)))

(fn GetRightDeck
  (return (Variables|Decks|GetRightDeck)))

(fn GetCardDecks
  (return (Utilities|Array|MakeArray (Variables|Decks|GetCard0) (Variables|Decks|GetCard1) (Variables|Decks|GetCard2) (Variables|Decks|GetCard3) (Variables|Decks|GetCard4))))

(fn DidIWin
  (if (Default|Empty (Variables|Decks|GetPlayerDeck))
    (bind _array_element (Utilities|Array|ForEachLoopwithBreak (CallFunction|GetCardDecks) :!label _label)
      (:LoopBody
        (if (not (Default|Empty _array_element))
          (goto _label Break)))
      (:Completed
        (return (Default|Empty _array_element))))
    (else
      (return false))))

(fn GetLeftDeck
  (return (Variables|Decks|GetLeftDeck)))